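; BP_GameMode runs the game's stage flow: start, kill-count progress, stage clear, game over and restart.
; It broadcasts each state change through event dispatchers, incrementing the kill count on every monster death and signaling stage clear when it equals the target.
; A separate event streams in SubLevel02 without blocking, while restart reopens the main level and then fires the game-start dispatcher.
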(event `LoadLevel`
  ; 서브 레벨 로드
  (`GameplayStatics.LoadStreamLevelBySoftObjectPtr` "/Game/Maps/Game/SubLevel02.SubLevel02" true))

(event `GameStart`
  ; 게임 시작 이벤트
  (`self.OnGameStart`)
  (`self.OnKillCountUpdated` (`self.CurKills`) (`self.TargetKills`)))

(event `MonsterKilled`
  ; 몬스터 죽었을 때 게임 모드 처리
  (bind _result (`/Engine/EditorBlueprintResources/StandardMacros.IncrementInt` (`self.CurKills`))
    (:`  `
      (`self.OnKillCountUpdated` _result (`self.TargetKills`))
      (if (== (`self.CurKills`) (`self.TargetKills`))
        (`self.OnStageClear`)))))

(event `GameOver`
  (`self.OnGameOver`))

(event `RestartGame`
  (`GameplayStatics.OpenLevelBySoftObjectPtr` "/Game/Maps/Game/MainLevel.MainLevel")
  (`self.OnGameStart`))

(fn `UserConstructionScript`)