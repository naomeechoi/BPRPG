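; Bear monster enemy with a Locomotion, Chase, Attack and Dead state machine that sets walk speed and mirrors state to the AI Blackboard.
; Sight perception of the player starts a chase, which drops back to Locomotion when the target gets too far.
; An HP controller component takes damage, updates the HP bar and triggers death.
; Attack collision is enabled only during attack check windows; timelines drive hit-flash and death-dissolve material parameters.
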(event `ReceiveOnDead`
  (bind _mesh (`self.Mesh`))
  ; Dead 이벤트 바인딩
  (`self.UpdateState` "NewEnumerator3")
  (`PrimitiveComponent.SetCollisionEnabled` (`self.CapsuleComponent`) "NoCollision")
  (`KismetSystemLibrary.Delay` 2.0)
  (bind (_direction _dissolve _hitvalue) (`Timeline|DeathEffect` :!via `PlayFromStart`)
    (:`Update`
      (`MeshComponent.SetScalarParameterValueOnMaterials` _mesh "Dissolve" _dissolve)
      (`MeshComponent.SetScalarParameterValueOnMaterials` _mesh "HitValue" _hitvalue)
      (if (>= _dissolve 1.0)
        (`self.K2_DestroyActor`)))))

(event `self.ReceiveBeginPlay`
  (`|ExecutionSequence`
    (:`then_0`
      ; 시작시 어택 콜리전 끄기
      (`PrimitiveComponent.SetCollisionEnabled` (`self.AttackCollision`) "NoCollision"))
    (:`then_1`
      ; Dead 이벤트 바인딩
      (add `/Game/Blueprints/Components/BP_HPController.OnDeadEvent` (`self.BP_HPController`) (delegate `ReceiveOnDead`)))
    (:`then_2`
      ; HP 이벤트 바인딩
      (add `/Game/Blueprints/Components/BP_HPController.OnHpChanged` (`self.BP_HPController`) (delegate `ReceiveOnHPChagned`)))
    (:`then_3`
      ; 데이터에서 맥스 HP 가져와 셋팅
      (`/Game/Blueprints/Components/BP_HPController.UpdateMaxHP` (`self.BP_HPController`) (`.MaxHP_11_3837F9964048E3E696795B809C03F30F` (break `/Game/Blueprints/Monster/Data/BP_MonsterLevelData` (`/Game/Blueprints/Monster/Data/BP_MonsterData.GetCurrentLevelData` (`self.BP_MonsterData`))))))))

(event `ReceiveOnHPChagned`
  (params (HP :type "Float (double-precision)") (MaxHP :type "Float (double-precision)"))
  ; HP 이벤트 바인딩
  (bind _aswbp_hpbar (cast `/Game/UI/WBP_HPBar` (`WidgetComponent.GetWidget` (`self.HPBar`))))
  (`/Game/UI/WBP_HPBar.UpdateHpPercent` _aswbp_hpbar (/ HP MaxHP)))

(event `self.ReceiveActorBeginOverlap`
  (params (OtherActor :type "Actor Object Reference"))
  ; 피격 효과
  (if (`self.ActorHasTag` OtherActor "PlayerWeapon")
    (bind (_direction _hitvalue) (`Timeline|HitEffect` :!via `PlayFromStart`)
      (:`Update`
        (`MeshComponent.SetScalarParameterValueOnMaterials` (`self.Mesh`) "HitValue" _hitvalue)))))

(event `self.ReceiveTick`
  (params (DeltaSeconds :type "Float (single-precision)"))
  (switch `/Game/Blueprints/Monster/EBearState` (`self.State_BP`)
    (:`NewEnumerator0`
      (`self.OnLocomotion`))
    (:`NewEnumerator1`
      (`self.OnChase`))
    (:`NewEnumerator2`
      (`self.OnAttack`))
    (:`NewEnumerator3`
      (`self.OnDead`))))

(event `self.ReceiveAnyDamage`
  (params (Damage :type "Float (single-precision)") (DamageType :type "DamageType Object Reference") (InstigatedBy :type "Controller Object Reference") (DamageCauser :type "Actor Object Reference"))
  ; 대미지 처리
  (`/Game/Blueprints/Components/BP_HPController.ReceiveDamage` (`self.BP_HPController`) Damage)
  (`self.TurnToTarget` (`self.GetOwner` DamageCauser)))

(event `self.AIPerception.OnTargetPerceptionUpdated`
  (params (Actor :type "Actor Object Reference") (Stimulus :type "AIStimulus Structure"))
  ; 시야 감지
  (if (`.bSuccessfullySensed` (break `AIStimulus` Stimulus))
    (if (`|EnumEquality` (`self.State_BP`) "NewEnumerator0")
      (if (`self.ActorHasTag` Actor "Player")
        (`BlackboardComponent.SetValueAsObject` (`AIBlueprintHelperLibrary.GetBlackboard` null) (`self.TargetPlayerKey`) Actor)
        (bind _asbp_character (cast `/Game/Blueprints/Character/BP_Character` Actor))
        (if (`|EnumInequality` (`/Game/Blueprints/Character/BP_Character.state_BP` _asbp_character) "NewEnumerator2")
          (`self.UpdateState` "NewEnumerator1"))))))

(event `UpdateState`
  (params (NewState :type "/Game/Blueprints/Monster/EBearState Enum" :default "NewEnumerator0"))
  (bind _charactermovement (`self.CharacterMovement`))
  ; 몬스터 상태 변경 이벤트
  (if (not (`|EnumEquality` (`self.State_BP`) "NewEnumerator3"))
    (bind _output_get (set `self.State_BP` NewState))
    (`BlackboardComponent.SetValueAsEnum` (`AIBlueprintHelperLibrary.GetBlackboard` null) (`self.StateKey`) _output_get)
    (switch `/Game/Blueprints/Monster/EBearState` (`self.State_BP`)
      (:`NewEnumerator0`
        (set `CharacterMovementComponent.MaxWalkSpeed` 200.0 _charactermovement))
      (:`NewEnumerator1`
        (set `CharacterMovementComponent.MaxWalkSpeed` 300.0 _charactermovement))
      (:`NewEnumerator2`
        (set `CharacterMovementComponent.MaxWalkSpeed` 0.0 _charactermovement :!label _label))
      (:`NewEnumerator3`
        (goto _label)))))

(event `OnAttackChcekStart`
  ; 공격 판정 시작 종료
  (`PrimitiveComponent.SetCollisionEnabled` (`self.AttackCollision`) "QueryOnly"))

(event `OnAttackChcekEnd`
  ; 공격 판정 시작 종료
  (`PrimitiveComponent.SetCollisionEnabled` (`self.AttackCollision`) "NoCollision"))

(event `self.AttackCollision.OnComponentBeginOverlap`
  (params (OverlappedComponent :type "PrimitiveComponent Object Reference") (OtherActor :type "Actor Object Reference") (OtherComp :type "PrimitiveComponent Object Reference") (OtherBodyIndex :type Integer) (bFromSweep :type Boolean) (SweepResult :type "HitResult Structure (by ref)"))
  (`GameplayStatics.ApplyDamage` OtherActor (`self.Base Damage`) (`self.GetController`) self))

(fn `OnAttack`
  (bind _asbp_character (cast `/Game/Blueprints/Character/BP_Character` (`BlackboardComponent.GetValueAsObject` (`AIBlueprintHelperLibrary.GetBlackboard` null) (`self.TargetPlayerKey`))))
  (if (`|EnumEquality` (`/Game/Blueprints/Character/BP_Character.state_BP` _asbp_character) "NewEnumerator2")
    (`self.UpdateState` "NewEnumerator0")))

(fn `OnChase`
  (bind _asactor (cast `Actor` (`BlackboardComponent.GetValueAsObject` (`AIBlueprintHelperLibrary.GetBlackboard` null) (`self.TargetPlayerKey`))))
  (if (> (`KismetMathLibrary.Vector_Distance` (`self.K2_GetActorLocation` _asactor) (`self.K2_GetActorLocation`)) 400.0)
    (`self.UpdateState` "NewEnumerator0")))

(fn `OnDead`)

(fn `OnLocomotion`)

(fn `TurnToTarget`
  (params (TargetPlayer :type "Actor Object Reference"))
  (bind (_returnvalue_roll _returnvalue_pitch _returnvalue_yaw) (`KismetMathLibrary.BreakRotator` (`KismetMathLibrary.MakeRotFromX` (- (`self.K2_GetActorLocation` TargetPlayer) (`self.K2_GetActorLocation`)))))
  (`self.K2_SetActorRotation` (`KismetMathLibrary.MakeRotator` 0.0 0.0 _returnvalue_yaw)))

(fn `UserConstructionScript`)