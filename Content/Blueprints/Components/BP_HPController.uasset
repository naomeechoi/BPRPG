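; BP_HPController is a health component that tracks current and maximum HP and handles incoming damage.
; HP starts full on BeginPlay, and UpdateMaxHP sets a new maximum and refills HP without broadcasting a change.
; ReceiveDamage ignores negative damage or already-depleted HP, subtracts damage and signals OnHpChanged.
; At zero or below it clamps HP and signals OnDeadEvent, so the change signal can carry negative HP.
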(event `self.ReceiveBeginPlay`
  (set `self.HP` (`self.MaxHP`)))

(event `UpdateMaxHP`
  (params (MaxHP :type "Float (double-precision)"))
  (bind _output_get (set `self.MaxHP` MaxHP))
  (set `self.HP` _output_get))

(event `ReceiveDamage`
  (params (Damage :type "Float (double-precision)"))
  ; 대미지 처리 과정 - Dead 이벤트도 발행
  (if (>= Damage 0.0)
    (if (> (`self.HP`) 0.0)
      (bind _output_get (set `self.HP` (- (`self.HP`) Damage)))
      (`self.OnHpChanged` (`self.HP`) (`self.MaxHP`))
      (if (<= _output_get 0.0)
        (set `self.HP` 0.0)
        (`self.OnDeadEvent`)))))